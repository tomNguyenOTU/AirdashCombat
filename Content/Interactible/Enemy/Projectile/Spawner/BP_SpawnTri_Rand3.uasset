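; Projectile spawner that launches a volley of charging actors at the player from random positions.
; Each LeftRightArray entry rolls a point in a Y/Z rectangle around the spawner, on its X plane.
; The actor spawns behind that point along the line to the player, with a charge target far along that line toward the player.
; It fires on BeginPlay, then either repeats on a timer if LoopThisSpawner is set or destroys itself.
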(event EventBeginPlay
  (CallFunction|Spawn)
  (if (Variables|Default|GetloopThisSpawner)
    (Utilities|Time|SetTimerbyFunctionName 0 "Spawn" 5.0 true)
    (else
      (Actor|DestroyActor))))

(fn ConstructionScript)

(fn Spawn
  (bind _returnvalue (Transformation|GetActorLocation))
  (bind _output_get (LocalVariables|SetinstanceFarLeft (Math|Vector|MakeVector (.x _returnvalue) (- (.y _returnvalue) 1.2e+03) (- (.z _returnvalue) 4e+02))))
  (LocalVariables|SetinstanceFarRight (Math|Vector|MakeVector (.x _output_get) (+ (.y _returnvalue) 1.2e+03) (+ (.z _returnvalue) 4e+02)))
  (for _array_element (LocalVariables|GetleftRightArray)
    (while (or (Utilities|Operators|EqualEqual :A (LocalVariables|GetrandomPosition)) false)
      (LocalVariables|SetrandomPosition (Math|Vector|MakeVector (.x (LocalVariables|GetinstanceFarLeft)) (Math|Random|RandomFloatinRange (.y (LocalVariables|GetinstanceFarLeft)) (.y (LocalVariables|GetinstanceFarRight))) (Math|Random|RandomFloatinRange (.z (LocalVariables|GetinstanceFarLeft)) (.z (LocalVariables|GetinstanceFarRight))))))
    (Game|SpawnActorfromClass "/Game/Interactible/Enemy/BP_BasicEnemy_IgnorePlayer.BP_BasicEnemy_IgnorePlayer_C" (Math|Transform|MakeTransform (- (LocalVariables|GetrandomPosition) (* (Math|Vector|GetUnitDirection(Vector) (LocalVariables|GetrandomPosition) (Transformation|GetActorLocation (Game|Player|GetPlayerPawn 0))) 1e+03)) "0, 0, 0" "1.000000,1.000000,1.000000") "Undefined" "MultiplyWithRoot" 0 (Variables|Default|GetcontainedRoom) (+ (LocalVariables|GetrandomPosition) (* (Math|Vector|GetUnitDirection(Vector) (LocalVariables|GetrandomPosition) (Transformation|GetActorLocation (Game|Player|GetPlayerPawn 0))) 5e+03)) 1.5e+03 0)
    (LocalVariables|SetrandomPosition "0, 0, 0")))