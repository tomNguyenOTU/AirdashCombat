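; Basic enemy that charges the player's last sampled position once the player enters its detection volume.
; Tick moves it without sweep, clamped to the target; on arrival it re-targets an overlapping player or stops, with a zero vector meaning idle.
; Sphere contact damages and bounces the player; received damage depletes health until destruction, which notifies BP_GameManager.
; It records its containing room camera at spawn, and ResetToInstanced restores starting position, health and idle state.
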(event OnComponentBeginOverlap(playerDetection)
  (params (OverlappedComponent :type Primitive%20Component%20Object%20Reference) (OtherActor :type Actor%20Object%20Reference) (OtherComp :type Primitive%20Component%20Object%20Reference) (OtherBodyIndex :type Integer) (bFromSweep :type Boolean) (SweepResult :type Hit%20Result%20Structure%20%28by%20ref%29))
  (if (Utilities|Operators|EqualEqual :A (Variables|Default|GettargetForCharge))
    (bind _asbp_third_person_character (Utilities|Casting|CastToBP_ThirdPersonCharacter OtherActor))
    (Variables|Default|SettargetForCharge (Transformation|GetActorLocation _asbp_third_person_character))
    (CallFunction|PointtoTarget)))

(event OnComponentBeginOverlap(Sphere1)
  (params (OverlappedComponent :type Primitive%20Component%20Object%20Reference) (OtherActor :type Actor%20Object%20Reference) (OtherComp :type Primitive%20Component%20Object%20Reference) (OtherBodyIndex :type Integer) (bFromSweep :type Boolean) (SweepResult :type Hit%20Result%20Structure%20%28by%20ref%29))
  (bind _asbp_third_person_character (Utilities|Casting|CastToBP_ThirdPersonCharacter OtherActor))
  (Game|Damage|ApplyDamage _asbp_third_person_character 1.0 0 self)
  (Default|BounceInverseForce _asbp_third_person_character))

(event EventBeginPlay
  (bind _returnvalue (Transformation|GetActorLocation))
  (bind _asbp_game_manager (Utilities|Casting|CastToBP_GameManager (Game|GetGameState)))
  (bind _containedcamera (Default|GetContainedCamera _asbp_game_manager _returnvalue))
  (Variables|Default|SetContainedRoom _containedcamera)
  (Transformation|SetActorRotation "0.000000,-90.000000,0.000000")
  (Variables|Default|SetinstancedPosition _returnvalue)
  (Variables|Default|SetmaxHealth (Variables|Default|Gethealth)))

(event EventTick
  (params (DeltaSeconds :type Float%20%28single-precision%29))
  (bind _returnvalue (Transformation|GetActorLocation))
  (bind _playerdetection (Variables|Default|GetplayerDetection))
  (bind _overlappingactors (Collision|GetOverlappingActors _playerdetection "/Game/ThirdPerson/Blueprints/BP_ThirdPersonCharacter.BP_ThirdPersonCharacter_C" :!class /Script/Engine.PrimitiveComponent))
  (if (not (Utilities|Operators|EqualEqual :A (Variables|Default|GettargetForCharge)))
    (Transformation|SetActorLocation (Math|Vector|SelectVector (Variables|Default|GettargetForCharge) (+ (Transformation|GetActorLocation) (* (Math|Vector|GetUnitDirection(Vector) _returnvalue (Variables|Default|GettargetForCharge)) (Variables|Default|GetmoveSpeed) DeltaSeconds)) (> (Math|Vector|VectorLength (* (Math|Vector|GetUnitDirection(Vector) _returnvalue (Variables|Default|GettargetForCharge)) (Variables|Default|GetmoveSpeed) DeltaSeconds)) (Math|Vector|Distance(Vector) (Variables|Default|GettargetForCharge) _returnvalue))) false false)
    (if (Utilities|Operators|EqualEqual (Transformation|GetActorLocation) (Variables|Default|GettargetForCharge) 2.5)
      (if (== (Utilities|Array|Length _overlappingactors) 0)
        (Variables|Default|SettargetForCharge "0, 0, 0")
        (else
          (Variables|Default|SettargetForCharge (Transformation|GetActorLocation (Utilities|Array|Get(acopy) _overlappingactors)))
          (CallFunction|PointtoTarget))))))

(event Game|Damage|EventAnyDamage
  (params (Damage :type Float%20%28single-precision%29) (DamageType :type Damage%20Type%20Object%20Reference) (InstigatedBy :type Controller%20Object%20Reference) (DamageCauser :type Actor%20Object%20Reference))
  (Class|FMODBlueprintStatics|PlayEventatLocation "/Game/FMOD/Events/SFX/Player/Hit_Enemy.Hit_Enemy" (Transformation|GetActorTransform))
  (bind _output_get (Variables|Default|Sethealth (- (Variables|Default|Gethealth) Damage)))
  (if (<= _output_get 0.0)
    (Actor|DestroyActor)))

(event EventDestroyed
  (bind _asbp_game_manager (Utilities|Casting|CastToBP_GameManager (Game|GetGameState)))
  (Default|RemovePawn _asbp_game_manager self))

(fn ConstructionScript)

(fn PointtoTarget
  (bind _returnvalue (Transformation|GetActorLocation))
  (bind _targetforcharge (Variables|Default|GettargetForCharge))
  (bind _returnvalue_2 (Math|Rotator|FindLookatRotation (Math|Vector|MakeVector (.x _returnvalue) (.y _returnvalue) (.z _returnvalue)) (Math|Vector|MakeVector (.x _targetforcharge) (.y _targetforcharge) (.z _targetforcharge))))
  (bind _returnvalue_3 (+ (.pitch _returnvalue_2) 0.0))
  (Transformation|SetActorRotation (Math|Rotator|MakeRotator 0.0 (Math|Float|SelectFloat _returnvalue_3 (+ (* _returnvalue_3 -1.0) 1.8e+02) (<= (.yaw _returnvalue_2) 0.0)) -9e+01)))

(fn ResettoInstanced
  (Transformation|SetActorLocationAndRotation (Variables|Default|GetinstancedPosition) "0.000000,-90.000000,0.000000")
  (Variables|Default|Sethealth (Variables|Default|GetmaxHealth))
  (Variables|Default|SettargetForCharge "0, 0, 0"))