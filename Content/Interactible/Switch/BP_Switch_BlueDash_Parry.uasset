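; Child switch Blueprint that responds only to a player blue dash that also passes a blue parry check.
; Overlaps passing both component checks are forwarded to the parent switch's overlap logic.
; A timer set on BeginPlay calls ParryLoop, which has the parry component spawn an indicator on the Cube.
; Tick unpauses that timer while Active and pauses it otherwise.
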(event EventBeginPlay
  (Utilities|Time|SetTimerbyFunctionName 0 "ParryLoop" 5.0)
  (|CallParentFunction))

(event Collision|EventActorBeginOverlap
  (params (OtherActor :type Actor%20Object%20Reference))
  (bind _isbluedash (Default|CheckifPlayerBlueDash (Variables|Default|GetBP_Comp_CheckIfPlayer) OtherActor))
  (if _isbluedash
    (bind _parried (Default|BlueParryCheck (Variables|Default|GetBP_Comp_ParryComponent)))
    (if _parried
      (|CallParentFunction OtherActor))))

(event EventTick
  (params (DeltaSeconds :type Float%20%28single-precision%29))
  (if (Variables|Default|Getactive)
    (Class|KismetSystemLibrary|UnPauseTimer 0 "ParryLoop")
    (else
      (Class|KismetSystemLibrary|PauseTimer 0 "ParryLoop"))))

(fn ConstructionScript
  (|CallParentFunction))

(fn ParryLoop
  (Default|SpawnParryIndicator (Variables|Default|GetBP_Comp_ParryComponent) (Variables|Default|GetCube) "NewEnumerator2"))