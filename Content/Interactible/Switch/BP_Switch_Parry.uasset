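; BP_Switch_Parry is an interactible switch that the player deactivates with a blue dash parry.
; On overlap, a player-check component confirms the actor is the player in a blue dash, and the parry component runs its blue parry check on the Cube before Deactivate is called.
; The parent overlap logic still runs afterwards.
; A ParryLoop function has the parry component spawn a parry indicator attached to the Cube.
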(event EventBeginPlay
  (|CallParentFunction) ; This node is disabled and will not be called.\nDrag off pins to build functionality.
)

(event Collision|EventActorBeginOverlap
  (params (OtherActor :type Actor%20Object%20Reference))
  (bind _isbluedash (Default|CheckifPlayerBlueDash (Variables|Default|GetBP_Comp_CheckIfPlayer) OtherActor))
  (if _isbluedash
    (bind _parried (Default|BlueParryCheck (Variables|Default|GetBP_Comp_ParryComponent) (Variables|Default|GetCube)))
    (if _parried
      (CallFunction|Deactivate)))
  (|CallParentFunction OtherActor))

(event EventTick
  (params (DeltaSeconds :type Float%20%28single-precision%29))
  (|CallParentFunction DeltaSeconds) ; This node is disabled and will not be called.\nDrag off pins to build functionality.
)

(fn ConstructionScript
  (|CallParentFunction))

(fn ParryLoop
  (Default|SpawnParryIndicator (Variables|Default|GetBP_Comp_ParryComponent) (Variables|Default|GetCube) "NewEnumerator5"))