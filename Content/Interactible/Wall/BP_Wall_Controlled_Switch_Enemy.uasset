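; Switch-controlled wall Blueprint that temporarily disappears and restores itself after a delay.
; DelayedRespawn toggles on Active: it disables collision, visibility and damageability, then sets a timer by function name to call itself after RespawnTimer.
; The second pass restores all three and clears the timer, and both passes play the Interactable_DestroyAttack audio event at the wall's location.
; The initial trigger for DelayedRespawn is outside these graphs.
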(fn ConstructionScript)

(fn DelayedRespawn
  (bind _staticmesh (Variables|Default|GetStaticMesh))
  (if (Variables|Default|Getactive)
    (Collision|SetCollisionEnabled _staticmesh "NoCollision")
    (Rendering|SetVisibility _staticmesh false false)
    (Variables|Actor|SetbCanBeDamaged false)
    (Variables|Default|Setactive false)
    (Utilities|Time|SetTimerbyFunctionName 0 "DelayedRespawn" (Variables|Default|GetrespawnTimer))
    (else
      (Collision|SetCollisionEnabled _staticmesh "QueryAndPhysics")
      (Rendering|SetVisibility _staticmesh true false)
      (Variables|Actor|SetbCanBeDamaged true)
      (Variables|Default|Setactive true)
      (Utilities|Time|ClearTimerbyFunctionName 0 "DelayedRespawn")))
  (Class|FMODBlueprintStatics|PlayEventatLocation "/Game/FMOD/Events/SFX/Object/Interactable_DestroyAttack.Interactable_DestroyAttack" (Transformation|GetActorTransform)))