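; BP_ButtonPrompt is a level object that shows a button prompt on a plane, switching its material to match the current input device.
; BeginPlay applies the gamepad material by default and binds to the controller-changed delegate of BP_ThirdPersonCharacter.
; The delegate handler picks the gamepad or non-gamepad material through IsUsingGamepad.
; Tick runs the same check, so the material is reassigned every frame regardless of the delegate.
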(event Custom|ReceiveControllerChangedDelegate_Event
  (params (Pawn :type Pawn%20Object%20Reference) (OldController :type Controller%20Object%20Reference) (NewController :type Controller%20Object%20Reference))
  (bind _materials (Variables|Default|GetMaterials))
  (bind _plane (Variables|Default|GetPlane))
  (if (CallFunction|IsUsingGamepad?)
    (Rendering|Material|SetMaterial _plane 0 (Utilities|Array|Get(acopy) _materials))
    (else
      (Rendering|Material|SetMaterial _plane 0 (Utilities|Array|Get(acopy) _materials 1)))))

(event EventBeginPlay
  (bind _asbp_third_person_character (Utilities|Casting|CastToBP_ThirdPersonCharacter (Game|Player|GetPlayerPawn 0)))
  (EventDispatchers|AssignReceiveControllerChangedDelegate _asbp_third_person_character (delegate Custom|ReceiveControllerChangedDelegate_Event))
  (Rendering|Material|SetMaterial (Variables|Default|GetPlane) 0 (Utilities|Array|Get(acopy) (Variables|Default|GetMaterials))))

(event EventTick
  (params (DeltaSeconds :type Float%20%28single-precision%29))
  (bind _materials (Variables|Default|GetMaterials))
  (bind _plane (Variables|Default|GetPlane))
  (if (CallFunction|IsUsingGamepad?)
    (Rendering|Material|SetMaterial _plane 0 (Utilities|Array|Get(acopy) _materials))
    (else
      (Rendering|Material|SetMaterial _plane 0 (Utilities|Array|Get(acopy) _materials 1)))))

(fn ConstructionScript)