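; BP_Switch_Stand is a floor or stand switch that the third-person character toggles by overlapping its box, driving a linked ControlledWall.
; ToggleSwitch flips SwitchOn, swaps the cube between red and the basic wall material, and calls DelayedRespawn on the wall for both states.
; Switching on starts a ResetTime timer that calls ToggleSwitch again to revert; switching off clears it.
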(event OnComponentBeginOverlap(Box)
  (params (OverlappedComponent :type Primitive%20Component%20Object%20Reference) (OtherActor :type Actor%20Object%20Reference) (OtherComp :type Primitive%20Component%20Object%20Reference) (OtherBodyIndex :type Integer) (bFromSweep :type Boolean) (SweepResult :type Hit%20Result%20Structure%20%28by%20ref%29))
  (Utilities|Casting|CastToBP_ThirdPersonCharacter OtherActor)
  (CallFunction|ToggleSwitch))

(event EventBeginPlay)

(event Collision|EventActorBeginOverlap
  (params (OtherActor :type Actor%20Object%20Reference)))

(event EventTick
  (params (DeltaSeconds :type Float%20%28single-precision%29)))

(fn ConstructionScript)

(fn ResetMaterial
  (CallFunction|ToggleSwitch))

(fn ToggleSwitch
  (bind _output_get (Variables|Default|SetswitchOn (not (Variables|Default|GetswitchOn))))
  (if _output_get
    (Rendering|Material|SetMaterial (Variables|Default|GetCube) 0 "/Game/Red.Red")
    (Utilities|Time|SetTimerbyFunctionName 0 "ToggleSwitch" (Variables|Default|GetresetTime))
    (else
      (Rendering|Material|SetMaterial (Variables|Default|GetCube) 0 "/Game/StarterContent/Materials/M_Basic_Wall.M_Basic_Wall")
      (Utilities|Time|ClearTimerbyFunctionName 0 "ToggleSwitch")))
  (Default|DelayedRespawn (Variables|Default|GetcontrolledWall)))