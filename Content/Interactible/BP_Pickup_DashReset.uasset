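; Pickup that resets the player's dash on overlap, then hides itself and respawns after a delay.
; Overlap with BP_ThirdPersonCharacter calls ResetDash, runs DelayedRespawn and plays the Interactable_DashReset event at the pickup's location.
; DelayedRespawn toggles on Active, disabling collision and visibility and setting a timer on itself, which restores both after RespawnTimer.
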(event Collision|EventActorBeginOverlap
  (params (OtherActor :type Actor%20Object%20Reference))
  ;[0.15 0.15 0.15 0.5] cast to player; reset dash then destroy
  (bind _asbp_third_person_character (Utilities|Casting|CastToBP_ThirdPersonCharacter OtherActor))
  (Default|ResetDash _asbp_third_person_character)
  (CallFunction|DelayedRespawn)
  (Class|FMODBlueprintStatics|PlayEventatLocation "/Game/FMOD/Events/SFX/Object/Interactable_DashReset.Interactable_DashReset" (Transformation|GetActorTransform)))

(fn ConstructionScript)

(fn DelayedRespawn
  (bind _spherecollision (Variables|Default|GetSphereCollision))
  (bind _spheremesh (Variables|Default|GetSphereMesh))
  (if (Variables|Default|Getactive)
    (Collision|SetCollisionEnabled _spheremesh "NoCollision")
    (Collision|SetCollisionEnabled _spherecollision "NoCollision")
    (Rendering|SetVisibility _spherecollision false true)
    (Variables|Default|Setactive false)
    (Utilities|Time|SetTimerbyFunctionName 0 "DelayedRespawn" (Variables|Default|GetrespawnTimer))
    (else
      (Collision|SetCollisionEnabled _spheremesh "QueryAndPhysics")
      (Collision|SetCollisionEnabled _spherecollision "QueryAndPhysics")
      (Rendering|SetVisibility _spherecollision true true)
      (Variables|Default|Setactive true))))