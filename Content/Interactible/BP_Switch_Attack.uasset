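; Attack-activated switch that toggles whenever it takes any damage and drives a linked wall.
; ToggleSwitch flips the state, swaps the cube between red and basic wall materials, and calls DelayedRespawn on ControlledWall in both directions.
; Switching on starts a named timer that re-runs ToggleSwitch after ResetTime to switch it back off, and switching off clears that timer.
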(event EventBeginPlay)

(event Collision|EventActorBeginOverlap
  (params (OtherActor :type Actor%20Object%20Reference)))

(event EventTick
  (params (DeltaSeconds :type Float%20%28single-precision%29)))

(event Game|Damage|EventAnyDamage
  (params (Damage :type Float%20%28single-precision%29) (DamageType :type Damage%20Type%20Object%20Reference) (InstigatedBy :type Controller%20Object%20Reference) (DamageCauser :type Actor%20Object%20Reference))
  (CallFunction|ToggleSwitch))

(fn ConstructionScript)

(fn ResetMaterial
  (CallFunction|ToggleSwitch))

(fn ToggleSwitch
  (bind _output_get (Variables|Default|SetswitchOn (not (Variables|Default|GetswitchOn))))
  (if _output_get
    (Rendering|Material|SetMaterial (Variables|Default|GetCube) 0 "/Game/Red.Red")
    (Utilities|Time|SetTimerbyFunctionName 0 "ToggleSwitch" (Variables|Default|GetresetTime))
    (else
      (Rendering|Material|SetMaterial (Variables|Default|GetCube) 0 "/Game/StarterContent/Materials/M_Basic_Wall.M_Basic_Wall")
      (Utilities|Time|ClearTimerbyFunctionName 0 "ToggleSwitch")))
  (Default|DelayedRespawn (Variables|Default|GetcontrolledWall)))