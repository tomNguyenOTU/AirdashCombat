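; Pickup that resets the player character's dash when it is deactivated.
; BeginPlay sets its interaction type, and the Deactivate override plays a sound event at its location, calls ResetDash on the player pawn, then disables and hides the collision sphere.
; The Activate override restores the sphere's collision and visibility, with both overrides finishing by calling the parent implementation.
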(event EventBeginPlay
  (Variables|Default|SetinteractionType "NewEnumerator3"))

(fn ConstructionScript)

(fn Deactivate
  (bind _spherecollision (Variables|Default|GetSphereCollision))
  (Class|FMODBlueprintStatics|PlayEventatLocation "/Game/FMOD/Events/SFX/Object/Interactable_DashReset.Interactable_DashReset" (Transformation|GetActorTransform))
  (bind _asbp_third_person_character (Utilities|Casting|CastToBP_ThirdPersonCharacter (Game|Player|GetPlayerPawn 0)))
  (Default|ResetDash _asbp_third_person_character)
  (Collision|SetCollisionEnabled _spherecollision "NoCollision")
  (Rendering|SetVisibility _spherecollision false true)
  (|CallParentFunction))

(fn Activate
  (bind _spherecollision (Variables|Default|GetSphereCollision))
  (Collision|SetCollisionEnabled _spherecollision "QueryAndPhysics")
  (Rendering|SetVisibility _spherecollision true true)
  (|CallParentFunction))