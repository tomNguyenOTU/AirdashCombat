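; Interactible wall that can be switched between a solid, damageable state and a hidden, passable one.
; WallOff runs only while active, disabling the mesh's collision, visibility and damage, then playing a destroy sound event at the actor's location.
; Reset restores all three and marks the wall active again.
; Activate and Deactivate overrides call Reset and WallOff respectively before passing on to the parent implementation.
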(fn ConstructionScript)

(fn WallOff
  (bind _staticmesh (Variables|Default|GetStaticMesh))
  (if (Variables|Default|Getactive)
    (Collision|SetCollisionEnabled _staticmesh "NoCollision")
    (Rendering|SetVisibility _staticmesh false true)
    (Variables|Default|SetbCanBeDamaged false)
    (Variables|Default|Setactive false)
    (Class|FMODBlueprintStatics|PlayEventatLocation "/Game/FMOD/Events/SFX/Object/Interactable_DestroyAttack.Interactable_DestroyAttack" (Transformation|GetActorTransform))))

(fn Reset
  (bind _staticmesh (Variables|Default|GetStaticMesh))
  (Collision|SetCollisionEnabled _staticmesh "QueryAndPhysics")
  (Rendering|SetVisibility _staticmesh true true)
  (Variables|Default|SetbCanBeDamaged true)
  (Variables|Default|Setactive true))

(fn Activate
  (CallFunction|Reset)
  (|CallParentFunction))

(fn Deactivate
  (CallFunction|WallOff)
  (|CallParentFunction))