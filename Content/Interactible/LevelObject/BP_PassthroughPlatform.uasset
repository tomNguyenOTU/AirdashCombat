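; One-way platform that the player passes through from below and stands on from above.
; Pawn collision starts ignored and switches to blocking when the Collision volume detects an overlap while the player is above BoxMesh, storing the platform in the character's PlatformTemp.
; The player's exit disables blocking and clears that reference, with Tick also disabling it when no character overlaps.
; CollisionOff is exposed for the player Blueprint to call.
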(event OnComponentBeginOverlap(Collision)
  (params (OverlappedComponent :type Primitive%20Component%20Object%20Reference) (OtherActor :type Actor%20Object%20Reference) (OtherComp :type Primitive%20Component%20Object%20Reference) (OtherBodyIndex :type Integer) (bFromSweep :type Boolean) (SweepResult :type Hit%20Result%20Structure%20%28by%20ref%29))
  (bind _returnvalue (Game|GetPlayerCharacter 0))
  (bind _charactermovement (Variables|/Script/Engine.Character|GetCharacterMovement _returnvalue))
  (bind _returnvalue_2 (Class|PawnMovementComponent|GetPawnOwner _charactermovement))
  ;[0.15 0.15 0.15 0.5] check for player
  (bind _asbp_third_person_character (Utilities|Casting|CastToBP_ThirdPersonCharacter _returnvalue_2))
  (if (> (.z (Transformation|GetActorLocation _returnvalue_2)) (.z (Transformation|GetWorldLocation (Variables|Default|GetBoxMesh))))
    (Collision|SetCollisionResponsetoChannel (Variables|Default|GetBoxMesh) "ECC_Pawn" "ECR_Block")
    ;[0.15 0.15 0.15 0.5] add to player var
    (bind _asbp_third_person_character_2 (Utilities|Casting|CastToBP_ThirdPersonCharacter OtherActor))
    (Variables|/Game/ThirdPerson/Blueprints/BP_ThirdPersonCharacter.BP_ThirdPersonCharacter_C|SetplatformTemp _asbp_third_person_character_2 self)))

(event OnComponentEndOverlap(Collision)
  (params (OverlappedComponent :type Primitive%20Component%20Object%20Reference) (OtherActor :type Actor%20Object%20Reference) (OtherComp :type Primitive%20Component%20Object%20Reference) (OtherBodyIndex :type Integer))
  ;[0.15 0.15 0.15 0.5] disable collision on play/when player leaves collisionbox
  (if (== OtherActor (Game|GetPlayerCharacter 0))
    (CallFunction|CollisionOff)
    ;[0.15 0.15 0.15 0.5] remove player's platform var
    (bind _asbp_third_person_character (Utilities|Casting|CastToBP_ThirdPersonCharacter OtherActor))
    (Variables|/Game/ThirdPerson/Blueprints/BP_ThirdPersonCharacter.BP_ThirdPersonCharacter_C|SetplatformTemp _asbp_third_person_character 0)))

(event EventTick
  (params (DeltaSeconds :type Float%20%28single-precision%29))
  (if (Utilities|Enum|Equal(Enum) (Collision|GetCollisionResponsetoChannel (Variables|Default|GetBoxMesh) "ECC_Pawn") "ECR_Block")
    (bind _asbp_third_person_character (Utilities|Casting|CastToBP_ThirdPersonCharacter (Game|GetPlayerCharacter 0)))
    (if (not (> (Utilities|Array|Length (Collision|GetOverlappingActors "/Game/ThirdPerson/Blueprints/BP_ThirdPersonCharacter.BP_ThirdPersonCharacter_C" :!class /Script/Engine.Actor)) 0))
      (CallFunction|CollisionOff))))

(event EventBeginPlay
  ;[0.15 0.15 0.15 0.5] disable collision on play/when player leaves collisionbox
  (CallFunction|CollisionOff)
  ;[0.15 0.15 0.15 0.5] remove player's platform var
  (bind _asbp_third_person_character (Utilities|Casting|CastToBP_ThirdPersonCharacter (stale OnComponentEndOverlap(Collision) OtherActor)))
  (Variables|/Game/ThirdPerson/Blueprints/BP_ThirdPersonCharacter.BP_ThirdPersonCharacter_C|SetplatformTemp _asbp_third_person_character 0))

(fn ConstructionScript)

(fn CollisionOff
  ;[0.15 0.15 0.15 0.5] callable from player BP
  (Collision|SetCollisionResponsetoChannel (Variables|Default|GetBoxMesh) "ECC_Pawn" "ECR_Ignore"))