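; Heavy-parry switch, an interactible that toggles when heavy damage passes its parry component's check.
; A five-second looping timer spawns a parry indicator on the Cube, and Tick pauses or resumes it according to the Active flag.
; Damage of the DT_Heavy type runs HeavyParryCheck on the Cube, and a successful check calls ActivateToggle.
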(event EventBeginPlay
  (Utilities|Time|SetTimerbyFunctionName 0 "ParryLoop" 5.0 true)
  (Variables|Default|SetinteractionType "NewEnumerator5")
  (|CallParentFunction))

(event Collision|EventActorBeginOverlap
  (params (OtherActor :type Actor%20Object%20Reference))
  (|CallParentFunction OtherActor))

(event EventTick
  (params (DeltaSeconds :type Float%20%28single-precision%29))
  (if (Variables|Default|Getactive)
    (Class|KismetSystemLibrary|UnPauseTimer 0 "ParryLoop")
    (else
      (Class|KismetSystemLibrary|PauseTimer 0 "ParryLoop"))))

(event Game|Damage|EventAnyDamage
  (params (Damage :type Float%20%28single-precision%29) (DamageType :type Damage%20Type%20Object%20Reference) (InstigatedBy :type Controller%20Object%20Reference) (DamageCauser :type Actor%20Object%20Reference))
  (if (== (Utilities|GetClass DamageType) "/Game/ThirdPerson/Blueprints/Attack/DT_Heavy.DT_Heavy_C")
    (bind _parried (Default|HeavyParryCheck (Variables|Default|GetBP_Comp_ParryComponent) (Variables|Default|GetCube)))
    (if _parried
      (CallFunction|ActivateToggle))))

(fn ConstructionScript
  (|CallParentFunction))

(fn ParryLoop
  (Default|SpawnParryIndicator (Variables|Default|GetBP_Comp_ParryComponent) (Variables|Default|GetCube) "NewEnumerator1"))