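; Base interactible actor that flips its Active state in response to the configured InteractionType: normal attack, heavy attack, blue airdash or contact.
; Damage events handle attacks, checking DT_Heavy for heavy ones, while overlaps use BPCompCheckIfPlayer to validate the player or blue dash.
; ActivateToggle alternates state when Toggleable and otherwise only deactivates.
; Deactivate can schedule reactivation by timer after ResetCooldown, though the toggle clears an ActivateToggle timer, not that Activate timer.
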(event Game|Damage|EventAnyDamage
  (params (Damage :type Float%20%28single-precision%29) (DamageType :type Damage%20Type%20Object%20Reference) (InstigatedBy :type Controller%20Object%20Reference) (DamageCauser :type Actor%20Object%20Reference))
  (switch Utilities|FlowControl|Switch|SwitchonE_InteractionType (Variables|Default|GetinteractionType)
    (:NewEnumerator0
      (CallFunction|ActivateToggle :!label _label))
    (:NewEnumerator1
      (if (== (Utilities|GetClass DamageType) "/Game/ThirdPerson/Blueprints/Attack/DT_Heavy.DT_Heavy_C")
        (goto _label)))))

(event Collision|EventActorBeginOverlap
  (params (OtherActor :type Actor%20Object%20Reference))
  (bind _bp_comp_checkifplayer (Variables|Default|GetBP_Comp_CheckIfPlayer))
  (switch Utilities|FlowControl|Switch|SwitchonE_InteractionType (Variables|Default|GetinteractionType)
    (:NewEnumerator2
      (bind _isbluedash (Default|CheckifPlayerBlueDash _bp_comp_checkifplayer OtherActor))
      (if _isbluedash
        (CallFunction|ActivateToggle :!label _label)))
    (:NewEnumerator3
      (bind _isplayer (Default|CheckifPlayer _bp_comp_checkifplayer OtherActor))
      (if _isplayer
        (goto _label)))))

(fn ConstructionScript)

(fn Activate
  (Variables|Default|Setactive true))

(fn Deactivate
  (Variables|Default|Setactive false)
  (if (Variables|Default|GetresetsOnCooldown)
    (Utilities|Time|SetTimerbyFunctionName 0 "Activate" (Variables|Default|GetresetCooldown))
    (else
      (Development|PrintString "222"))))

(fn ActivateToggle
  (if (Variables|Default|Gettoggleable)
    (Utilities|Time|ClearTimerbyFunctionName 0 "ActivateToggle")
    (if (Variables|Default|Getactive)
      (CallFunction|Deactivate)
      (else
        (CallFunction|Activate)))
    (else
      (CallFunction|Deactivate))))