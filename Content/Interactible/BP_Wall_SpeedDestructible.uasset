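; Speed-destructible wall that breaks when the player hits it while blue airdashing or moving faster than SpeedReq.
; Actor and both box overlaps share one check on the player character while the wall is Active.
; DelayedRespawn works as a toggle: it hides the mesh and Box and disables their collision, then sets a timer on itself to restore them after RespawnTimer.
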(event OnComponentBeginOverlap(Box1)
  (params (OverlappedComponent :type Primitive%20Component%20Object%20Reference) (OtherActor :type Actor%20Object%20Reference) (OtherComp :type Primitive%20Component%20Object%20Reference) (OtherBodyIndex :type Integer) (bFromSweep :type Boolean) (SweepResult :type Hit%20Result%20Structure%20%28by%20ref%29))
  (if (Variables|Default|Getactive)
    (Variables|Default|Setother OtherActor)
    ;[0.15 0.15 0.15 0.5] cast to player if able
    (bind _asbp_third_person_character (Utilities|Casting|CastToBP_ThirdPersonCharacter (Variables|Default|Getother)))
    ;[0.15 0.15 0.15 0.5] destroy if player is blue airdashing OR if velocity is above speed req (this should just be really fucking high)
    (if (or (Variables|/Game/ThirdPerson/Blueprints/BP_ThirdPersonCharacter.BP_ThirdPersonCharacter_C|GetblueAirdashing _asbp_third_person_character) (> (Math|Vector|VectorLength (Transformation|GetVelocity _asbp_third_person_character)) (Variables|Default|GetspeedReq)))
      (CallFunction|DelayedRespawn))))

(event OnComponentBeginOverlap(Box)
  (params (OverlappedComponent :type Primitive%20Component%20Object%20Reference) (OtherActor :type Actor%20Object%20Reference) (OtherComp :type Primitive%20Component%20Object%20Reference) (OtherBodyIndex :type Integer) (bFromSweep :type Boolean) (SweepResult :type Hit%20Result%20Structure%20%28by%20ref%29))
  (if (Variables|Default|Getactive)
    (Variables|Default|Setother OtherActor)
    ;[0.15 0.15 0.15 0.5] cast to player if able
    (bind _asbp_third_person_character (Utilities|Casting|CastToBP_ThirdPersonCharacter (Variables|Default|Getother)))
    ;[0.15 0.15 0.15 0.5] destroy if player is blue airdashing OR if velocity is above speed req (this should just be really fucking high)
    (if (or (Variables|/Game/ThirdPerson/Blueprints/BP_ThirdPersonCharacter.BP_ThirdPersonCharacter_C|GetblueAirdashing _asbp_third_person_character) (> (Math|Vector|VectorLength (Transformation|GetVelocity _asbp_third_person_character)) (Variables|Default|GetspeedReq)))
      (CallFunction|DelayedRespawn))))

(event Collision|EventActorBeginOverlap
  (params (OtherActor :type Actor%20Object%20Reference))
  ;[0.15 0.15 0.15 0.5] cast to player if able
  (if (Variables|Default|Getactive)
    (Variables|Default|Setother OtherActor)
    (bind _asbp_third_person_character (Utilities|Casting|CastToBP_ThirdPersonCharacter (Variables|Default|Getother)))
    ;[0.15 0.15 0.15 0.5] destroy if player is blue airdashing OR if velocity is above speed req (this should just be really fucking high)
    (if (or (Variables|/Game/ThirdPerson/Blueprints/BP_ThirdPersonCharacter.BP_ThirdPersonCharacter_C|GetblueAirdashing _asbp_third_person_character) (> (Math|Vector|VectorLength (Transformation|GetVelocity _asbp_third_person_character)) (Variables|Default|GetspeedReq)))
      (CallFunction|DelayedRespawn))))

(fn ConstructionScript)

(fn DelayedRespawn
  (bind _staticmesh (Variables|Default|GetStaticMesh))
  (bind _box (Variables|Default|GetBox))
  (if (Variables|Default|Getactive)
    (Collision|SetCollisionEnabled _staticmesh "NoCollision")
    (Rendering|SetVisibility _staticmesh false false)
    (Collision|SetCollisionEnabled _box "NoCollision")
    (Rendering|SetVisibility _box false false)
    (Variables|Default|Setactive false)
    (Utilities|Time|SetTimerbyFunctionName 0 "DelayedRespawn" (Variables|Default|GetrespawnTimer))
    (else
      (Collision|SetCollisionEnabled _staticmesh "QueryAndPhysics")
      (Rendering|SetVisibility _staticmesh true false)
      (Collision|SetCollisionEnabled _box "QueryAndPhysics")
      (Rendering|SetVisibility _box true false)
      (Variables|Default|Setactive true))))