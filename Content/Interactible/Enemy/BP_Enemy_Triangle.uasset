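; Triangle enemy Blueprint that idles by periodically turning around and attacks the player by moving toward them along Y.
; While active, Tick checks sight with a sphere overlap, absolute dot-product cone (covering front and back) and line trace.
; Detection results start delayed timers that switch the AI mode to attack or back to its default.
; It overrides the parent's idle and attack behaviors, using yaw flips for facing.
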(event EventBeginPlay
  (Transformation|SetActorRotation "0.000000,90.000000,0.000000")
  (Variables|Default|SetmaxHealth 5e+01)
  (Variables|Default|SetdefaultAIMode (Variables|Default|GetcurrentAIMode))
  (|CallParentFunction))

(event EventTick
  (params (DeltaSeconds :type Float%20%28single-precision%29))
  (bind _active (CallFunction|CheckifActive))
  (if _active
    (bind (_canseeplayer _playerpos) (CallFunction|CheckConeLook))
    (Variables|Default|SetplayerAt _playerpos)
    (if _canseeplayer
      (if (> (Class|KismetSystemLibrary|GetTimerRemainingTime 0 "DelayedAttackPlayer") 0.0)
        _
        (else
          (Utilities|Time|SetTimerbyFunctionName 0 "DelayedAttackPlayer" (Variables|Default|GetdetectDelay))))
      (elif (> (Class|KismetSystemLibrary|GetTimerRemainingTime 0 "DelayedReturnNormal") 0.0)
        _
        (else
          (Utilities|Time|SetTimerbyFunctionName 0 "DelayedReturnNormal" (Variables|Default|GetdetectDelay)))))
    (|CallParentFunction DeltaSeconds)
    (else
      (|CallParentFunction DeltaSeconds))))

(fn ConstructionScript
  (|CallParentFunction))

(fn CheckConeLook
  (bind _returnvalue (Transformation|GetActorLocation))
  (bind (_outactors _returnvalue_2) (Collision|SphereOverlapActors _returnvalue (Variables|Default|GetcheckRange) (Utilities|Array|MakeArray "ObjectTypeQuery3") "/Game/ThirdPerson/Blueprints/BP_ThirdPersonCharacter.BP_ThirdPersonCharacter_C"))
  (if _returnvalue_2
    (if (> (Math|Float|Absolute(Float) (Math|Vector|DotProduct (Transformation|GetActorForwardVector) (Math|Vector|Normalize (- (Transformation|GetActorLocation (Utilities|Array|Get(acopy) _outactors)) _returnvalue)))) 0.8)
      (bind _returnvalue_3 (Class|KismetSystemLibrary|LineTraceSinglebyProfile _returnvalue (Transformation|GetActorLocation (Utilities|Array|Get(acopy) _outactors)) "IgnoreOnlyPawn" false 0 "ForOneFrame" true))
      (if _returnvalue_3
        (return false (Variables|Default|GetplayerAt))
        (else
          (return true (Transformation|GetActorLocation (Utilities|Array|Get(acopy) _outactors)))))
      (else
        (return false (Variables|Default|GetplayerAt))))
    (else
      (return false (Variables|Default|GetplayerAt)))))

(fn RunAttackPlayer
  (if (> (.y (Transformation|GetActorLocation)) (.y (Variables|Default|GetplayerAt)))
    (Transformation|SetActorRotation "0.000000,-90.000000,0.000000")
    (else
      (Transformation|SetActorRotation "0.000000,90.000000,0.000000")))
  (Pawn|Input|AddMovementInput (Transformation|GetActorForwardVector) (Variables|Default|GetmoveSpeed) true)
  (|CallParentFunction))

(fn DelayedAttackPlayer
  (Variables|Default|SetcurrentAIMode "NewEnumerator4"))

(fn NewFunction)

(fn RunIdle
  (if (not (> (Class|KismetSystemLibrary|GetTimerRemainingTime 0 "TurnAround") 0.0))
    (Utilities|Time|SetTimerbyFunctionName 0 "TurnAround" (Math|Conversions|ToFloat(Integer) (Math|Random|RandomIntegerinRange 4 6)))))

(fn TurnAround
  (Transformation|SetActorRotation (Math|Rotator|MakeRotator 0.0 0.0 (* (.yaw (Transformation|GetActorRotation)) -1.0))))

(fn DelayedReturnNormal
  (Variables|Default|SetcurrentAIMode (Variables|Default|GetdefaultAIMode))
  (Utilities|Time|ClearTimerbyFunctionName 0 "DelayedReturnNormal"))