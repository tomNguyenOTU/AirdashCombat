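; BP_PassthroughPlatform is a one-way platform that toggles its box mesh between blocking and ignoring Pawns.
; Player overlap with the collision volume turns blocking on, after a short delay if below the mesh, and stores the platform on BP_ThirdPersonCharacter.
; End overlap and BeginPlay call CollisionOff, which the player Blueprint can also use.
; Tick calls the player's PassthroughPlatform when the mesh blocks without the player overlapping.
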(event OnComponentBeginOverlap(Collision)
  (params (OverlappedComponent :type Primitive%20Component%20Object%20Reference) (OtherActor :type Actor%20Object%20Reference) (OtherComp :type Primitive%20Component%20Object%20Reference) (OtherBodyIndex :type Integer) (bFromSweep :type Boolean) (SweepResult :type Hit%20Result%20Structure%20%28by%20ref%29))
  (bind _returnvalue (Game|GetPlayerCharacter 0))
  ;[0.15 0.15 0.15 0.5] check for player
  (if (== OtherActor _returnvalue)
    ;[0.15 0.15 0.15 0.5] delay if player is under platform
    (if (> (.z (Transformation|GetActorLocation _returnvalue)) (.z (Transformation|GetWorldLocation (Variables|Default|GetBoxMesh))))
      _
      (else
        (Utilities|FlowControl|Delay 0.2)))
    (Collision|SetCollisionResponsetoChannel (Variables|Default|GetBoxMesh) "ECC_Pawn" "ECR_Block")
    ;[0.15 0.15 0.15 0.5] add to player var
    (bind _asbp_third_person_character (Utilities|Casting|CastToBP_ThirdPersonCharacter OtherActor))
    (Variables|/Game/ThirdPerson/Blueprints/BP_ThirdPersonCharacter.BP_ThirdPersonCharacter_C|SetplatformTemp _asbp_third_person_character self)))

(event OnComponentEndOverlap(Collision)
  (params (OverlappedComponent :type Primitive%20Component%20Object%20Reference) (OtherActor :type Actor%20Object%20Reference) (OtherComp :type Primitive%20Component%20Object%20Reference) (OtherBodyIndex :type Integer))
  ;[0.15 0.15 0.15 0.5] disable collision on play/when player leaves collisionbox
  (if (== OtherActor (Game|GetPlayerCharacter 0))
    (CallFunction|CollisionOff)
    ;[0.15 0.15 0.15 0.5] remove player's platform var
    (bind _asbp_third_person_character (Utilities|Casting|CastToBP_ThirdPersonCharacter OtherActor))
    (Variables|/Game/ThirdPerson/Blueprints/BP_ThirdPersonCharacter.BP_ThirdPersonCharacter_C|SetplatformTemp _asbp_third_person_character 0)))

(event EventTick
  (params (DeltaSeconds :type Float%20%28single-precision%29))
  (if (Utilities|Enum|Equal(Enum) (Collision|GetCollisionResponsetoChannel (Variables|Default|GetBoxMesh) "ECC_Pawn") "ECR_Block")
    (bind _asbp_third_person_character (Utilities|Casting|CastToBP_ThirdPersonCharacter (Game|GetPlayerCharacter 0)))
    (if (not (Utilities|Array|ContainsItem (Collision|GetOverlappingActors 0 :!class /Script/Engine.Actor) _asbp_third_person_character))
      (Default|PassthroughPlatform _asbp_third_person_character))))

(event EventBeginPlay
  ;[0.15 0.15 0.15 0.5] disable collision on play/when player leaves collisionbox
  (CallFunction|CollisionOff)
  ;[0.15 0.15 0.15 0.5] remove player's platform var
  (bind _asbp_third_person_character (Utilities|Casting|CastToBP_ThirdPersonCharacter (stale OnComponentEndOverlap(Collision) OtherActor)))
  (Variables|/Game/ThirdPerson/Blueprints/BP_ThirdPersonCharacter.BP_ThirdPersonCharacter_C|SetplatformTemp _asbp_third_person_character 0))

(fn ConstructionScript)

(fn CollisionOff
  ;[0.15 0.15 0.15 0.5] callable from player BP
  (Collision|SetCollisionResponsetoChannel (Variables|Default|GetBoxMesh) "ECC_Pawn" "ECR_Ignore"))