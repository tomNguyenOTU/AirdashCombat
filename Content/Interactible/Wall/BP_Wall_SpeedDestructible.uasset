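; A wall that deactivates when the player hits it fast enough or while blue dashing.
; Overlaps on ExtCollision and BoxCollision both ask BPCompCheckIfPlayer whether the actor is a blue-dashing player or one moving above SpeedReq.
; Either check passing calls Deactivate.
; BeginPlay sets the wall's InteractionType.
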(event OnComponentBeginOverlap(ExtCollision)
  (params (OverlappedComponent :type Primitive%20Component%20Object%20Reference) (OtherActor :type Actor%20Object%20Reference) (OtherComp :type Primitive%20Component%20Object%20Reference) (OtherBodyIndex :type Integer) (bFromSweep :type Boolean) (SweepResult :type Hit%20Result%20Structure%20%28by%20ref%29))
  (bind _bp_comp_checkifplayer (Variables|Default|GetBP_Comp_CheckIfPlayer))
  (bind _isbluedash (Default|CheckifPlayerBlueDash _bp_comp_checkifplayer OtherActor))
  (bind _isbluedash_2 (Default|CheckifPlayerVelocity _bp_comp_checkifplayer OtherActor (Variables|Default|GetspeedReq)))
  (if (or _isbluedash_2 _isbluedash)
    (CallFunction|Deactivate)))

(event OnComponentBeginOverlap(BoxCollision)
  (params (OverlappedComponent :type Primitive%20Component%20Object%20Reference) (OtherActor :type Actor%20Object%20Reference) (OtherComp :type Primitive%20Component%20Object%20Reference) (OtherBodyIndex :type Integer) (bFromSweep :type Boolean) (SweepResult :type Hit%20Result%20Structure%20%28by%20ref%29))
  (bind _bp_comp_checkifplayer (Variables|Default|GetBP_Comp_CheckIfPlayer))
  (bind _isbluedash (Default|CheckifPlayerBlueDash _bp_comp_checkifplayer OtherActor))
  (bind _isbluedash_2 (Default|CheckifPlayerVelocity _bp_comp_checkifplayer OtherActor (Variables|Default|GetspeedReq)))
  (if (or _isbluedash_2 _isbluedash)
    (CallFunction|Deactivate)))

(event EventBeginPlay
  (Variables|Default|SetinteractionType "NewEnumerator5"))

(fn ConstructionScript)