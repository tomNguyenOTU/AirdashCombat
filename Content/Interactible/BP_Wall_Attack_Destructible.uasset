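; Destructible wall actor that breaks when it takes any damage and comes back after a delay.
; On damage it plays the Interactable_DestroyAttack audio event at its location and calls DelayedRespawn.
; DelayedRespawn toggles on the Active flag, hiding the mesh and disabling collision and damage, then re-arms itself by timer after RespawnTimer to restore all three.
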(event Game|Damage|EventAnyDamage
  (params (Damage :type Float%20%28single-precision%29) (DamageType :type Damage%20Type%20Object%20Reference) (InstigatedBy :type Controller%20Object%20Reference) (DamageCauser :type Actor%20Object%20Reference))
  (CallFunction|DelayedRespawn)
  (Class|FMODBlueprintStatics|PlayEventatLocation "/Game/FMOD/Events/SFX/Object/Interactable_DestroyAttack.Interactable_DestroyAttack" (Transformation|GetActorTransform)))

(fn ConstructionScript)

(fn DelayedRespawn
  (bind _staticmesh (Variables|Default|GetStaticMesh))
  (if (Variables|Default|Getactive)
    (Collision|SetCollisionEnabled _staticmesh "NoCollision")
    (Rendering|SetVisibility _staticmesh false false)
    (Variables|Actor|SetbCanBeDamaged false)
    (Variables|Default|Setactive false)
    (Utilities|Time|SetTimerbyFunctionName 0 "DelayedRespawn" (Variables|Default|GetrespawnTimer))
    (else
      (Collision|SetCollisionEnabled _staticmesh "QueryAndPhysics")
      (Rendering|SetVisibility _staticmesh true false)
      (Variables|Actor|SetbCanBeDamaged true)
      (Variables|Default|Setactive true))))