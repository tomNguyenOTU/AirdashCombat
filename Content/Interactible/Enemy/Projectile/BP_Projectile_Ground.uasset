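; BP_Projectile_Ground is an enemy projectile that flies in a straight line and hurts the player on contact.
; On spawn it attaches a shuriken Niagara effect to its box, offsets its roll and yaw by 90 degrees, and starts a lifetime timer that destroys it.
; Tick moves it along its forward vector at Speed without sweeping, and box overlap with the third-person character applies damage and triggers an inverse-force bounce.
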(event OnComponentBeginOverlap(Box)
  (params (OverlappedComponent :type Primitive%20Component%20Object%20Reference) (OtherActor :type Actor%20Object%20Reference) (OtherComp :type Primitive%20Component%20Object%20Reference) (OtherBodyIndex :type Integer) (bFromSweep :type Boolean) (SweepResult :type Hit%20Result%20Structure%20%28by%20ref%29))
  (bind _asbp_third_person_character (Utilities|Casting|CastToBP_ThirdPersonCharacter OtherActor))
  (Game|Damage|ApplyDamage OtherActor 1.0 0 self)
  (Default|BounceInverseForce _asbp_third_person_character))

(event EventBeginPlay
  (bind _returnvalue (Transformation|GetActorRotation))
  (Utilities|Time|SetTimerbyFunctionName 0 "KillSelf" (Variables|Default|Getlifetime))
  (Niagara|SpawnSystemAttached "/Game/VFXPackages/MixedVFX/Particles/Projectiles/NS_Shuriken_04.NS_Shuriken_04" (Variables|Default|GetBox) "None" "0, 0, 0" "0.000000,180.000000,180.000000" "KeepRelativeOffset" false)
  (Transformation|SetActorRotation (Math|Rotator|MakeRotator (+ (.roll _returnvalue) 9e+01) (.pitch _returnvalue) (+ (.yaw _returnvalue) 9e+01))))

(event EventTick
  (params (DeltaSeconds :type Float%20%28single-precision%29))
  (Transformation|SetActorLocation (+ (* DeltaSeconds (Variables|Default|Getspeed) (Transformation|GetActorForwardVector)) (Transformation|GetActorLocation)) false false))

(fn ConstructionScript)

(fn KillSelf
  (Actor|DestroyActor))