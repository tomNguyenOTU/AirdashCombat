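; BP_SpawnTriNew is a spawner actor that periodically creates triangle enemies at its own location.
; Two seconds after BeginPlay it spawns one, then a looping timer repeats the spawn every few seconds.
; Each BP_Enemy_Triangle always spawns with a default AI mode and hardcoded contained room, then gets a default controller, capsule physics simulation and enabled collision.
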(event EventBeginPlay
  (Utilities|FlowControl|Delay 2.0)
  (CallFunction|Spawn)
  (Utilities|Time|SetTimerbyFunctionName 0 "Spawn" 5.0 true))

(fn ConstructionScript)

(fn Spawn
  (bind _returnvalue (Game|SpawnActorfromClass "/Game/Interactible/Enemy/BP_Enemy_Triangle.BP_Enemy_Triangle_C" (Math|Transform|MakeTransform (Transformation|GetActorLocation) "0, 0, 0" "1.000000,1.000000,1.000000") "AlwaysSpawn" "MultiplyWithRoot" 0 "NewEnumerator0" (Variables|Default|Gethardcoderoom) "NewEnumerator0" 0))
  (Pawn|SpawnDefaultController _returnvalue)
  (Physics|SetSimulatePhysics (Variables|/Script/Engine.Character|GetCapsuleComponent _returnvalue) true)
  (Collision|SetActorEnableCollision _returnvalue true))