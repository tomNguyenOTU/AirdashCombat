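; BP_Switch is an interactable switch that controls a linked wall, passing its own activation and deactivation on to it.
; At BeginPlay it caches its mesh's original material alongside a red one and copies its cooldown reset settings to the wall.
; Activate and Deactivate drive the wall, swap the mesh to the original or red material respectively, then call the parent implementation.
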(event EventBeginPlay
  (bind _controlledwall (Variables|Default|GetcontrolledWall))
  (Variables|Default|SetMaterials (Utilities|Array|MakeArray (Rendering|Material|GetMaterial (Variables|Default|GetstaticMeshEditMat) 0) "/AnimationSharing/AnimSharingRed.AnimSharingRed"))
  (Variables|/Game/Interactible/BP_InteractibleBase.BP_InteractibleBase_C|SetresetsOnCooldown _controlledwall (Variables|Default|GetresetsOnCooldown))
  (Variables|/Game/Interactible/BP_InteractibleBase.BP_InteractibleBase_C|SetresetCooldown _controlledwall (Variables|Default|GetresetCooldown)))

(fn ConstructionScript)

(fn Deactivate
  (CallFunction|Deactivate (Variables|Default|GetcontrolledWall))
  (CallFunction|SetMaterialforMesh false)
  (|CallParentFunction))

(fn Activate
  (CallFunction|Activate (Variables|Default|GetcontrolledWall))
  (CallFunction|SetMaterialforMesh true)
  (|CallParentFunction))

(fn SetMaterialforMesh
  (params (OnOff :type Boolean))
  (bind _staticmesheditmat (Variables|Default|GetstaticMeshEditMat))
  (bind _materials (Variables|Default|GetMaterials))
  (if OnOff
    (Rendering|Material|SetMaterial _staticmesheditmat 0 (Utilities|Array|Get(acopy) _materials))
    (else
      (Rendering|Material|SetMaterial _staticmesheditmat 0 (Utilities|Array|Get(acopy) _materials 1)))))