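; BP_SpeedRing is a level object that launches the player character along its arrow when they enter its collision.
; On overlap it teleports the character to the collision's center, resets gravity and applies a launch that overrides existing velocity.
; It disables dashing and zeroes the air-dash timer, then resets the dash after a short delay.
; A Niagara burst and a ring sound event play at the ring's location.
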(event OnComponentBeginOverlap(Collision)
  (params (OverlappedComponent :type Primitive%20Component%20Object%20Reference) (OtherActor :type Actor%20Object%20Reference) (OtherComp :type Primitive%20Component%20Object%20Reference) (OtherBodyIndex :type Integer) (bFromSweep :type Boolean) (SweepResult :type Hit%20Result%20Structure%20%28by%20ref%29))
  (bind _collision (Variables|Default|GetCollision))
  (bind _returnvalue (Transformation|GetWorldLocation _collision))
  (bind _asbp_third_person_character (Utilities|Casting|CastToBP_ThirdPersonCharacter OtherActor))
  (Transformation|SetActorLocation _asbp_third_person_character (Transformation|GetWorldLocation (Variables|Default|GetCollision)) false true)
  (Default|ResetGravity _asbp_third_person_character 1.0)
  (Character|LaunchCharacter _asbp_third_person_character (* (Math|Vector|GetForwardVector (Variables|Default|GetArrow)) (Variables|Default|GetlaunchVelocity)) true true)
  (Variables|/Game/ThirdPerson/Blueprints/BP_ThirdPersonCharacter.BP_ThirdPersonCharacter_C|SetcanDash _asbp_third_person_character false)
  (Variables|/Game/ThirdPerson/Blueprints/BP_ThirdPersonCharacter.BP_ThirdPersonCharacter_C|SetbAirdashTimer _asbp_third_person_character 0.0)
  (Niagara|SpawnSystematLocation "/Game/VFXPackages/MixedVFX/Particles/Explosions/NS_ExplosionGroundMedium.NS_ExplosionGroundMedium" _returnvalue)
  (Class|FMODBlueprintStatics|PlayEventatLocation "/Game/FMOD/Events/SFX/Object/Interactable_Ring.Interactable_Ring" (Math|Conversions|ToTransform(Vector) _returnvalue))
  (Utilities|FlowControl|Delay 0.15)
  (Default|ResetDash _asbp_third_person_character))

(fn ConstructionScript)