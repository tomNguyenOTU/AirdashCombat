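; Ceiling spawner that drops staggered waves of charging actors from above its location within a contained room.
; On BeginPlay it spawns a wave, then either repeats on a looping timer or destroys itself.
; Each wave randomly starts at the far left or right, stepping inward and upward per array entry to form a diagonal targeted straight down, slightly faster from the right.
; The SpawnTri helper is not called here.
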(event Custom|spawnEvent
  (bind _returnvalue (Transformation|GetActorLocation))
  (Variables|Default|SetrandBool (Math|Random|RandomBool))
  (bind _output_get (Variables|Default|SetinstanceFarLeft (Math|Vector|MakeVector (.x _returnvalue) (- (.y _returnvalue) 1.2e+03) (+ (.z _returnvalue) 1e+03))))
  (Variables|Default|SetinstanceFarRight (Math|Vector|MakeVector (.x _output_get) (+ (.y _returnvalue) 1.2e+03) (.z _output_get)))
  (if (Variables|Default|GetrandBool)
    (for (_ _array_index) (Variables|Default|GetleftRightArray)
      (Game|SpawnActorfromClass "/Game/Interactible/Enemy/BP_BasicEnemy_IgnorePlayer.BP_BasicEnemy_IgnorePlayer_C" (Math|Transform|MakeTransform (Math|Vector|MakeVector (.x (Variables|Default|GetinstanceFarLeft)) (+ (.y (Variables|Default|GetinstanceFarLeft)) (* 200 _array_index)) (+ (.z (Variables|Default|GetinstanceFarLeft)) (* _array_index 4e+02))) "0, 0, 0" "1.000000,1.000000,1.000000") "Undefined" "MultiplyWithRoot" 0 (Variables|Default|GetcontainedRoom) (Math|Vector|MakeVector (.x (Variables|Default|GetinstanceFarLeft)) (+ (.y (Variables|Default|GetinstanceFarLeft)) (* 200 _array_index)) -1e+03) 1.5e+03 0))
    (else
      (for (_ _array_index_2) (Variables|Default|GetleftRightArray)
        (Game|SpawnActorfromClass "/Game/Interactible/Enemy/BP_BasicEnemy_IgnorePlayer.BP_BasicEnemy_IgnorePlayer_C" (Math|Transform|MakeTransform (Math|Vector|MakeVector (.x (Variables|Default|GetinstanceFarLeft)) (- (.y (Variables|Default|GetinstanceFarRight)) (* 200 _array_index_2)) (+ (.z (Variables|Default|GetinstanceFarLeft)) (* _array_index_2 4e+02))) "0, 0, 0" "1.000000,1.000000,1.000000") "Undefined" "MultiplyWithRoot" 0 (Variables|Default|GetcontainedRoom) (Math|Vector|MakeVector (.x (Variables|Default|GetinstanceFarLeft)) (- (.y (Variables|Default|GetinstanceFarRight)) (* 200 _array_index_2)) -1e+03) 1625.0 0)))))

(event EventBeginPlay
  (CallFunction|Spawn)
  (if (Variables|Default|GetloopThisSpawner)
    (Utilities|Time|SetTimerbyFunctionName 0 "Spawn" 5.0 true)
    (else
      (Actor|DestroyActor))))

(fn ConstructionScript)

(fn Spawn
  (CallFunction|SpawnEvent))

(fn SpawnTri
  (params (Location :type Vector) (Target :type Vector))
  (Game|SpawnActorfromClass "/Game/Interactible/Enemy/BP_BasicEnemy_IgnorePlayer.BP_BasicEnemy_IgnorePlayer_C" (Math|Transform|MakeTransform Location "0, 0, 0" "1.000000,1.000000,1.000000") "Undefined" "MultiplyWithRoot" 0 0 Target 0))