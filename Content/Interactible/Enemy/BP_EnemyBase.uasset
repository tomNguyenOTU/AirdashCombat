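; Base enemy Blueprint that damages the player on overlap, takes damage and is destroyed at zero health.
; It resolves its room camera from the game manager and runs a mode-switched AI only while unstunned and that room's camera is current.
; Blue-dash overlaps and heavy hits go through parry checks that can trigger a stun.
; Stun and AI behaviors are empty stubs, and a reset restores spawn position and health.
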(event Custom|InitRoomCamEnemy
  (bind _containedcamera (Default|GetContainedCamera (stale EventBeginPlay _asbp_game_manager) (stale EventBeginPlay _output_get)))
  (Variables|Default|SetContainedRoom _containedcamera))

(event Collision|EventActorBeginOverlap
  (params (OtherActor :type Actor%20Object%20Reference))
  (if (not (Variables|Default|GetisStunned))
    (bind _isbluedash (Default|CheckifPlayerBlueDash (Variables|Default|GetBP_Comp_CheckIfPlayer) OtherActor))
    (if _isbluedash
      (bind _parried (Default|BlueParryCheck (Variables|Default|GetBP_Comp_ParryComponent) (Variables|Default|GetparryAttach)))
      (if _parried
        (CallFunction|DoStun)
        (else
          (bind _isplayer (Default|CheckifPlayer (Variables|Default|GetBP_Comp_CheckIfPlayer) OtherActor :!label _label))
          (if _isplayer
            (Game|Damage|ApplyDamage OtherActor 1.0 0 self))))
      (else
        (goto _label)))))

(event EventBeginPlay
  (Variables|Default|Sethealth (Variables|Default|GetmaxHealth))
  (bind _output_get (Variables|Default|SetinstancedPosition (Transformation|GetActorLocation)))
  (bind _asbp_game_manager (Utilities|Casting|CastToBP_GameManager (Game|GetGameState)))
  (EventDispatchers|BindEventtoLateBeginPlay _asbp_game_manager (delegate Custom|InitRoomCamEnemy)))

(event EventDestroyed
  (bind _asbp_game_manager (Utilities|Casting|CastToBP_GameManager (Game|GetGameState)))
  (Default|RemovePawn _asbp_game_manager self))

(event Game|Damage|EventAnyDamage
  (params (Damage :type Float%20%28single-precision%29) (DamageType :type Damage%20Type%20Object%20Reference) (InstigatedBy :type Controller%20Object%20Reference) (DamageCauser :type Actor%20Object%20Reference))
  (Class|FMODBlueprintStatics|PlayEventatLocation "/Game/FMOD/Events/SFX/Player/Hit_Enemy.Hit_Enemy" (Transformation|GetActorTransform))
  (if (== (Utilities|GetClass DamageType) "/Game/ThirdPerson/Blueprints/Attack/DT_Heavy.DT_Heavy_C")
    (bind _parried (Default|HeavyParryCheck (Variables|Default|GetBP_Comp_ParryComponent) (Variables|Default|GetparryAttach)))
    (if _parried
      (CallFunction|DoStun)))
  (bind _output_get (Variables|Default|Sethealth (- (Variables|Default|Gethealth) Damage)))
  (if (<= _output_get 0.0)
    (CallFunction|EnemyDeath)))

(event EventTick
  (params (DeltaSeconds :type Float%20%28single-precision%29))
  (if (not (Variables|Default|GetisStunned))
    (bind _asbp_game_manager (Utilities|Casting|CastToBP_GameManager (Game|GetGameState)))
    (bind _output_get (Variables|Default|SetplayerInRoom (== (Variables|/Game/ThirdPerson/Blueprints/Manager/BP_GameManager.BP_GameManager_C|GetcurrentCam _asbp_game_manager) (Variables|Default|GetcontainedRoom))))
    (if _output_get
      (CallFunction|RunAI))))

(fn ConstructionScript)

(fn EnemyDeath
  (Actor|DestroyActor))

(fn ResettoInstanced
  (Transformation|SetActorLocationAndRotation (Variables|Default|GetinstancedPosition) "0.000000,-90.000000,0.000000")
  (Variables|Default|Sethealth (Variables|Default|GetmaxHealth))
  (Variables|Default|SetisStunned false))

(fn ResetStun
  (Variables|Default|SetisStunned false))

(fn DoStun)

(fn CheckifActive
  (return (and (not (Variables|Default|GetisStunned)) (Variables|Default|GetplayerInRoom))))

(fn RunAI
  (switch Utilities|FlowControl|Switch|SwitchonE_EnemyBehavior (Variables|Default|GetcurrentAIMode)
    (:NewEnumerator0
      (CallFunction|RunIdle))
    (:NewEnumerator1
      (CallFunction|RunStand))
    (:NewEnumerator2
      (CallFunction|RunPatrol))
    (:NewEnumerator4
      (CallFunction|RunAttackPlayer))))

(fn RunIdle)

(fn RunStand)

(fn RunPatrol)

(fn RunAttackPlayer)